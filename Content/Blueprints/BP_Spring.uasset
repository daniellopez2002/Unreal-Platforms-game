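; BP_Spring is a spring pad that launches BP_Robot upward when the robot hits its box.
; The hit sets the robot's jumping flag and plays a timeline that moves the spring between its cached start position and a fixed world Z height.
; Each timeline update also reapplies the launch using the Impulse value.
; When the timeline finishes, the spring returns to its original location.
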(event OnComponentHit(Box)
  (params (HitComponent :type Primitive%20Component%20Object%20Reference) (OtherActor :type Actor%20Object%20Reference) (OtherComp :type Primitive%20Component%20Object%20Reference) (NormalImpulse :type Vector :default "0, 0, 0") (Hit :type Hit%20Result%20Structure%20%28by%20ref%29))
  (bind _originalspringlocation (Variables|Default|GetoriginalSpringLocation))
  (bind _asbp_robot (Utilities|Casting|CastToBP_Robot OtherActor))
  (Variables|/Game/Blueprints/BP_Robot.BP_Robot_C|SetIsjumping _asbp_robot true)
  (bind _springheight (Timeline|Timeline_Spring PlayFromStart)
    (:Update
      (Transformation|SetWorldLocation (Variables|Default|GetSpring) (Math|Vector|Lerp(Vector) (Variables|Default|GetoriginalSpringLocation) (Math|Vector|MakeVector (.x _originalspringlocation) (.y _originalspringlocation) -4e+01) _springheight) true false)
      (Character|LaunchCharacter _asbp_robot (Math|Vector|MakeVector 0.0 0.0 (Variables|Default|GetImpulse)) false false))
    (:Finished
      (Transformation|SetWorldLocation (Variables|Default|GetSpring) (Variables|Default|GetoriginalSpringLocation) true false))))

(event EventBeginPlay
  (Variables|Default|SetoriginalSpringLocation (Transformation|GetWorldLocation (Variables|Default|GetSpring))))

(event Collision|EventActorBeginOverlap
  (params (OtherActor :type Actor%20Object%20Reference)))

(event EventTick
  (params (DeltaSeconds :type Float%20%28single-precision%29)))

(fn ConstructionScript)