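; BP_CheckPoint is a checkpoint flag that unlocks the first time a BP_Robot enters its sphere trigger.
; On that overlap it registers itself with the robot through AddCheckpoint and sets IsUnlock, so later overlaps with the robot have no effect.
; Unlocking also plays an explosion particle attached to the EmmisorReference component and swaps the static mesh to a red flag.
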(event OnComponentBeginOverlap(Sphere)
  (params (OverlappedComponent :type Primitive%20Component%20Object%20Reference) (OtherActor :type Actor%20Object%20Reference) (OtherComp :type Primitive%20Component%20Object%20Reference) (OtherBodyIndex :type Integer) (bFromSweep :type Boolean) (SweepResult :type Hit%20Result%20Structure%20%28by%20ref%29))
  (bind _asbp_robot (Utilities|Casting|CastToBP_Robot OtherActor))
  (if (not (Variables|Default|GetIsUnlock))
    (Default|AddCheckpoint _asbp_robot self)
    (Variables|Default|SetIsUnlock true)
    (Effects|SpawnEmitterAttached "/Game/Realistic_Starter_VFX_Pack_Vol2/Particles/Explosion/P_Explosion_Big_B.P_Explosion_Big_B" (Variables|Default|GetEmmisorReference) "None")
    (Components|StaticMesh|SetStaticMesh (Variables|Default|GetStaticMesh) "/Game/Assets/Models/red/flag_A_red.flag_A_red")))

(event EventBeginPlay)

(event Collision|EventActorBeginOverlap
  (params (OtherActor :type Actor%20Object%20Reference)))

(event EventTick
  (params (DeltaSeconds :type Float%20%28single-precision%29)))

(fn ConstructionScript)