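; Movable platform actor meant to slide along Z or X, as chosen by AxisZ.
; BeginPlay stores the start location and sets the timeline play rate from Speed; nothing in the graph calls Play on the timeline.
; Timeline updates lerp with sweep to an absolute Z of Distance, or to X offset by Distance.
; IsInvese negates the resulting world position (whole vector for Z, only X for X) rather than the offset.
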(event EventBeginPlay
  (Variables|Default|SetOriginalLocation (Transformation|GetActorLocation))
  (Components|Timeline|SetPlayRate (Variables|Default|GetTimeline_MovablePlatform) (Variables|Default|GetSpeed)))

(event Collision|EventActorBeginOverlap
  (params (OtherActor :type Actor%20Object%20Reference)))

(event EventTick
  (params (DeltaSeconds :type Float%20%28single-precision%29)))

(fn ConstructionScript)