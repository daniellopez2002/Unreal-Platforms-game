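; Player robot character for a side-scrolling platformer, with left/right movement, limited multi-jump and checkpoint respawning.
; Enhanced Input drives movement and jumps, with air jumps using LaunchCharacter plus a spark effect, while Tick traces downward to measure floor distance.
; Overlapping BP_DeadZone explodes the robot, teleports it to the last checkpoint and counts the death.
; Points, kill count, visited checkpoints and level reached persist through BP_SaveGame in one save slot.
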(event OnComponentBeginOverlap(CapsuleComponent)
  (params (OverlappedComponent :type Primitive%20Component%20Object%20Reference) (OtherActor :type Actor%20Object%20Reference) (OtherComp :type Primitive%20Component%20Object%20Reference) (OtherBodyIndex :type Integer) (bFromSweep :type Boolean) (SweepResult :type Hit%20Result%20Structure%20%28by%20ref%29))
  (Utilities|FlowControl|Sequence
    (:then_0
      (if (== (Utilities|GetClass OtherActor) "/Game/Blueprints/BP_DeadZone.BP_DeadZone_C")
        (CallFunction|KillRobot)))
    (:then_1
      (if true
        _))))

(event Custom|AddPoints
  (params (Points :type Integer))
  (Variables|Default|SetPoints (+ Points (Variables|Default|GetPoints))))

(event Custom|KillRobot
  (Rendering|SetVisibility (Variables|Character|GetMesh) false false)
  (Effects|SpawnEmitteratLocation "/Game/Realistic_Starter_VFX_Pack_Vol2/Particles/Explosion/P_Explosion_Big_A.P_Explosion_Big_A" (Transformation|GetActorLocation))
  (Audio|PlaySound2D "/Game/Assets/Sound/SFX_explosion.SFX_explosion" 1.0 1.0 0.0 0 0)
  (Utilities|FlowControl|Delay 1.0)
  (Transformation|Teleport (Variables|Default|GetCheckPointPosition) "0, 0, 0")
  (Rendering|SetVisibility (Variables|Character|GetMesh) true false)
  (Math|Integer|IncrementInt (Variables|Default|GetKillsCounter)))

(event Custom|EndLevel
  (bind _savegame (Variables|Default|GetSaveGame))
  (Utilities|IsValid _savegame
    (:Is%20Valid
      (Variables|/Game/Blueprints/BP_SaveGame.BP_SaveGame_C|SetKillCounter _savegame (Variables|Default|GetKillsCounter))
      (Variables|/Game/Blueprints/BP_SaveGame.BP_SaveGame_C|SetPoints _savegame (Variables|Default|GetPoints))
      (SaveGame|SaveGametoSlot _savegame "Slot 1")
      (Rendering|SetVisibility (Variables|Character|GetMesh) false false)
      (Effects|SpawnEmitteratLocation "/Game/Realistic_Starter_VFX_Pack_Vol2/Particles/Explosion/P_Explosion_Big_A.P_Explosion_Big_A" (Transformation|GetActorLocation))
      (Audio|PlaySound2D "/Game/Assets/Sound/SFX_explosion.SFX_explosion" 1.0 1.0 0.0 0 0))))

(event Input|EnhancedActionEvents|EnhancedInputActionJump
  (params (ActionValue :type Boolean) (ElapsedSeconds :type Float%20%28double-precision%29) (TriggeredSeconds :type Float%20%28double-precision%29) (InputAction :type Input%20Action%20Object%20Reference :default "/Game/Inputs/Jump.Jump"))
  (:Triggered
    (if (> (Variables|Default|GetMaxJumpCount) (Variables|Default|GetCurrentJumpCount))
      (if (Variables|Default|GetIsjumping)
        (Character|LaunchCharacter (Math|Vector|MakeVector 0.0 0.0 (Variables|Default|GetJumpForce)) false false)
        (bind _returnvalue (Effects|SpawnEmitterAttached "/Game/Realistic_Starter_VFX_Pack_Vol2/Particles/Sparks/P_Sparks_E.P_Sparks_E" (Variables|Default|GetReferenceJumpVFX) "None" "0, 0, 0" "0, 0, 0" "5.000000,5.000000,5.000000"))
        (else
          (Variables|Default|SetIsjumping true)
          (Utilities|FlowControl|Delay 0.5)
          (Character|Jump)))
      (Math|Integer|IncrementInt (Variables|Default|GetCurrentJumpCount)
        (:%20%20
          (Utilities|FlowControl|Delay 1.0)
          (Utilities|IsValid _returnvalue
            (:Is%20Valid
              (Components|DestroyComponent _returnvalue)))))))
  (:Canceled
    (Character|StopJumping :!label _label))
  (:Completed
    (goto _label)))

(event Input|EnhancedActionEvents|EnhancedInputActionMoveRightLeft
  (params (ActionValue :type Float%20%28double-precision%29) (ElapsedSeconds :type Float%20%28double-precision%29) (TriggeredSeconds :type Float%20%28double-precision%29) (InputAction :type Input%20Action%20Object%20Reference :default "/Game/Inputs/MoveRightLeft.MoveRightLeft"))
  (bind _mesh (Variables|Character|GetMesh))
  (if (> ActionValue 0.0)
    (Transformation|SetWorldRotation _mesh "0.000000,-90.000000,0.000000" false false)
    (else
      (Transformation|SetWorldRotation _mesh "0.000000,90.000000,0.000000" false false)))
  (Pawn|Input|AddMovementInput (Transformation|GetActorForwardVector) (* ActionValue (Variables|Default|GetSpeed)) false))

(event EventBeginPlay
  (Utilities|FlowControl|Sequence
    (:then_0
      (bind _returnvalue (SaveGame|DoesSaveGameExist "Slot 1"))
      (if _returnvalue
        (bind _returnvalue_2 (SaveGame|LoadGamefromSlot "Slot 1"))
        (bind _asbp_save_game (Utilities|Casting|CastToBP_SaveGame _returnvalue_2))
        (Variables|Default|SetSaveGame _asbp_save_game)
        (else
          (bind _returnvalue_3 (SaveGame|CreateSaveGameObject "/Game/Blueprints/BP_SaveGame.BP_SaveGame_C"))
          (Variables|Default|SetSaveGame _returnvalue_3))))
    (:then_1
      (Variables|Default|SetCheckPointPosition (Transformation|GetActorLocation))
      (Input|AddMappingContext (PlayerController|LocalPlayerSubsystems|GetEnhancedInputLocalPlayerSubsystem (Game|GetPlayerController 0)) "/Game/Inputs/InputMappingContext.InputMappingContext" 0 "(bIgnoreAllPressedKeysUntilRelease=True,bForceImmediately=False,bNotifyUserSettings=False)")
      (Variables|/Script/Engine.CharacterMovementComponent|SetJumpZVelocity (Variables|Character|GetCharacterMovement) (Variables|Default|GetJumpForce)))
    (:then_2
      (Utilities|IsValid (Variables|Default|GetSaveGame)
        (:Is%20Valid
          (Variables|Default|SetPoints (Variables|/Game/Blueprints/BP_SaveGame.BP_SaveGame_C|GetPoints (Variables|Default|GetSaveGame)))
          (Variables|Default|SetKillsCounter (Variables|/Game/Blueprints/BP_SaveGame.BP_SaveGame_C|GetKillCounter (Variables|Default|GetSaveGame)))
          (SaveGame|SaveGametoSlot (Variables|Default|GetSaveGame) "Slot 1"))))))

(event EventTick
  (params (DeltaSeconds :type Float%20%28single-precision%29))
  (bind _referencejumpvfx (Variables|Default|GetReferenceJumpVFX))
  (bind _returnvalue (Transformation|GetWorldLocation _referencejumpvfx))
  (Utilities|FlowControl|Sequence
    (:then_0
      (bind (_outhit _returnvalue_2) (Collision|LineTraceByChannel _returnvalue (+ _returnvalue (Math|Vector|MakeVector 0.0 0.0 -1e+03)) "TraceTypeQuery1" false 0 "None"))
      (if _returnvalue_2
        (Variables|Default|SetFloorDistance (Math|Vector|VectorLength (- (.TraceStart (Collision|BreakHitResult _outhit)) (.ImpactPoint (Collision|BreakHitResult _outhit)))))))))

(event EventOnLanded
  (params (Hit :type Hit%20Result%20Structure%20%28by%20ref%29))
  (Variables|Default|SetCurrentJumpCount 0)
  (Variables|Default|SetIsjumping false))

(fn ConstructionScript)

(fn AddCheckpoint
  (params (CheckPointReference :type BP%20Check%20Point%20Object%20Reference))
  (Variables|Default|SetCheckPointPosition (Transformation|GetActorLocation CheckPointReference))
  (bind _returnvalue (SaveGame|DoesSaveGameExist "Slot 1"))
  (if _returnvalue
    (bind _returnvalue_2 (SaveGame|LoadGamefromSlot "Slot 1"))
    (bind _asbp_save_game (Utilities|Casting|CastToBP_SaveGame _returnvalue_2)
      (:then
        (Variables|/Game/Blueprints/BP_SaveGame.BP_SaveGame_C|SetPoints _asbp_save_game (+ (Variables|/Game/Blueprints/BP_SaveGame.BP_SaveGame_C|GetPoints _asbp_save_game) (Variables|Default|GetPoints)))
        (Variables|/Game/Blueprints/BP_SaveGame.BP_SaveGame_C|SetPlayerLocation _asbp_save_game "0, 0, 0")
        (Utilities|Array|Add (Variables|/Game/Blueprints/BP_SaveGame.BP_SaveGame_C|GetCheckPointsVisited _asbp_save_game) CheckPointReference)
        (Variables|/Game/Blueprints/BP_SaveGame.BP_SaveGame_C|SetKillCounter _asbp_save_game (Variables|Default|GetKillsCounter))
        (SaveGame|SaveGametoSlot _asbp_save_game "Slot 1"))
      (:CastFailed
        (bind _returnvalue_3 (SaveGame|CreateSaveGameObject "/Game/Blueprints/BP_SaveGame.BP_SaveGame_C" :!label _label))
        (Variables|/Game/Blueprints/BP_SaveGame.BP_SaveGame_C|SetPoints _returnvalue_3 (Variables|Default|GetPoints))
        (Variables|/Game/Blueprints/BP_SaveGame.BP_SaveGame_C|SetPlayerLocation _returnvalue_3 (Variables|Default|GetCheckPointPosition))
        (Utilities|Array|Add (Variables|/Game/Blueprints/BP_SaveGame.BP_SaveGame_C|GetCheckPointsVisited _returnvalue_3) CheckPointReference)
        (Variables|/Game/Blueprints/BP_SaveGame.BP_SaveGame_C|SetKillCounter _returnvalue_3 (Variables|Default|GetKillsCounter))
        (SaveGame|SaveGametoSlot _returnvalue_3 "Slot 1")))
    (else
      (goto _label))))

(fn Startlevel
  (params (Level%20Index :type Integer))
  (bind _returnvalue (SaveGame|DoesSaveGameExist "Slot 1"))
  (if _returnvalue
    (bind _returnvalue_2 (SaveGame|LoadGamefromSlot "Slot 1"))
    (bind _asbp_save_game (Utilities|Casting|CastToBP_SaveGame _returnvalue_2))
    (Variables|/Game/Blueprints/BP_SaveGame.BP_SaveGame_C|SetLevelReach _asbp_save_game Level%20Index)
    (SaveGame|SaveGametoSlot _asbp_save_game "Slot 1")
    (else
      (bind _returnvalue_3 (SaveGame|CreateSaveGameObject "/Game/Blueprints/BP_SaveGame.BP_SaveGame_C"))
      (Variables|/Game/Blueprints/BP_SaveGame.BP_SaveGame_C|SetLevelReach _returnvalue_3 Level%20Index)
      (SaveGame|SaveGametoSlot _returnvalue_3 "Slot 1"))))