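; BP_TrapPlatform is a trap platform whose spikes move vertically when a BP_Robot steps into its trigger box and kill the robot they hit.
; The box overlap plays a timeline that lerps the spikes from their BeginPlay location along Z with a swept move, then resets them when it finishes.
; A hit on the spikes component calls KillRobot on the robot.
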(event OnComponentBeginOverlap(Box)
  (params (OverlappedComponent :type Primitive%20Component%20Object%20Reference) (OtherActor :type Actor%20Object%20Reference) (OtherComp :type Primitive%20Component%20Object%20Reference) (OtherBodyIndex :type Integer) (bFromSweep :type Boolean) (SweepResult :type Hit%20Result%20Structure%20%28by%20ref%29))
  (bind _originallocationspikes (Variables|Default|GetOriginalLocationSpikes))
  (Utilities|Casting|CastToBP_Robot OtherActor)
  (bind _spikesheight (Timeline|Timeline_Spike PlayFromStart)
    (:Update
      (Transformation|SetWorldLocation (Variables|Default|GetSpikes) (Math|Vector|Lerp(Vector) (Variables|Default|GetOriginalLocationSpikes) (Math|Vector|MakeVector (.x _originallocationspikes) (.y _originallocationspikes) 0.0) _spikesheight) true false))
    (:Finished
      (Transformation|SetWorldLocation (Variables|Default|GetSpikes) (Variables|Default|GetOriginalLocationSpikes) true false))))

(event OnComponentHit(Spikes)
  (params (HitComponent :type Primitive%20Component%20Object%20Reference) (OtherActor :type Actor%20Object%20Reference) (OtherComp :type Primitive%20Component%20Object%20Reference) (NormalImpulse :type Vector :default "0, 0, 0") (Hit :type Hit%20Result%20Structure%20%28by%20ref%29))
  (bind _asbp_robot (Utilities|Casting|CastToBP_Robot OtherActor))
  (Default|KillRobot _asbp_robot))

(event EventBeginPlay
  (Variables|Default|SetOriginalLocationSpikes (Transformation|GetWorldLocation (Variables|Default|GetSpikes))))

(event Collision|EventActorBeginOverlap
  (params (OtherActor :type Actor%20Object%20Reference)))

(event EventTick
  (params (DeltaSeconds :type Float%20%28single-precision%29)))

(fn ConstructionScript)