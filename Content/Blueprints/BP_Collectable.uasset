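; BP_Collectable is a spinning pickup that awards its Points value to a BP_Robot that touches it.
; Tick adds a fixed yaw step to the static mesh each frame, so spin speed depends on frame rate.
; The mesh's overlap event calls AddPoints on the robot, spawns a fireflies effect at its location and hides the mesh.
; The actor is not destroyed and its collision is left unchanged.
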(event OnComponentBeginOverlap(StaticMesh)
  (params (OverlappedComponent :type Primitive%20Component%20Object%20Reference) (OtherActor :type Actor%20Object%20Reference) (OtherComp :type Primitive%20Component%20Object%20Reference) (OtherBodyIndex :type Integer) (bFromSweep :type Boolean) (SweepResult :type Hit%20Result%20Structure%20%28by%20ref%29))
  (bind _asbp_robot (Utilities|Casting|CastToBP_Robot OtherActor))
  (Default|AddPoints _asbp_robot (Variables|Default|GetPoints))
  (Effects|SpawnEmitteratLocation "/Game/Realistic_Starter_VFX_Pack_Vol2/Particles/Environment/P_Fireflies.P_Fireflies" (Transformation|GetActorLocation _asbp_robot))
  (Rendering|SetVisibility (Variables|Default|GetStaticMesh) false false))

(event EventBeginPlay)

(event Collision|EventActorBeginOverlap
  (params (OtherActor :type Actor%20Object%20Reference)))

(event EventTick
  (params (DeltaSeconds :type Float%20%28single-precision%29))
  (bind _staticmesh (Variables|Default|GetStaticMesh))
  (Transformation|SetWorldRotation _staticmesh (Math|Rotator|MakeRotator 0.0 0.0 (+ (.yaw (Transformation|GetWorldRotation _staticmesh)) 0.5)) false false))

(fn ConstructionScript)